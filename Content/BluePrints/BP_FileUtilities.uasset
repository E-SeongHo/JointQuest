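; BP_FileUtilities is a set of helper functions that store per-user profile and knee game data as JSON files.
; GetUserData builds a UserData path under the project directory from the username, then returns age, body length and the knee game's max score and angle.
; GetJson creates and saves a default profile when the file is missing.
; UpdateJson sets one field on the passed object and writes it back to disk.
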(fn `GetJson`
  (params (Path :type String))
  (returns (JsonObject :type "JsonObjectWrapper Structure"))
  (bind _filepath (make `FilePath` Path))
  (if (`BlueprintPathsLibrary.FileExists` Path)
    (bind _outjsonobject (`JsonBlueprintFunctionLibrary.FromFile` _filepath))
    (return _outjsonobject)
    (else
      (bind _outjsonobject_2 (`JsonBlueprintFunctionLibrary.FromString` "{\"username\":\"\", \"age\":\"20\", \"body_length\":\"null\", \"knee_game\":{\"max_score\": \"0\", \"max_angle\":\"0\"}}"))
      (`JsonBlueprintFunctionLibrary.ToFile` _outjsonobject_2 _filepath)
      (bind _outjsonobject_3 (`JsonBlueprintFunctionLibrary.FromFile` _filepath))
      (return _outjsonobject_3))))

(fn `GetUserData`
  (params (Username :type String))
  (returns (JsonPath :type "FilePath Structure") (UserData :type "JsonObjectWrapper Structure") (BodyLength :type String) (Age :type String) (MaxScore :type String) (MaxAngle :type String))
  (locals (JsonPath :type "FilePath Structure") (user_data :type "JsonObjectWrapper Structure") (body_length :type String) (age :type String) (max_score :type String) (max_angle :type String))
  (bind _userdatapathstring (`self.GetUserDataPathString` Username))
  (bind _jsonobject (`self.GetJson` _userdatapathstring))
  (`|ExecutionSequence`
    (:`then_0`
      (bind _outvalue (`|GetJsonField` _jsonobject "body_length"))
      (bind _outjsonstring (`JsonBlueprintFunctionLibrary.ToString` _outvalue)))
    (:`then_1`
      (bind _outvalue_2 (`|GetJsonField` _jsonobject "age")))
    (:`then_2`
      (bind _outvalue_3 (`|GetJsonField` _jsonobject "knee_game"))
      (`|ExecutionSequence`
        (:`then_0`
          (bind _outvalue_4 (`|GetJsonField` _outvalue_3 "max_score")))
        (:`then_1`
          (bind _outvalue_5 (`|GetJsonField` _outvalue_3 "max_angle")))))
    (:`then_3`
      (return (make `FilePath` _userdatapathstring) _jsonobject _outjsonstring _outvalue_2 _outvalue_4 _outvalue_5))))

(fn `GetUserDataPathString`
  (params (Username :type String))
  (returns (UserDataPathString :type String))
  (return (`KismetStringLibrary.Concat_StrStr` (`KismetSystemLibrary.GetProjectDirectory`) "/UserData/" Username ".json")))

(fn `UpdateJson`
  (params (JsonObject :type "JsonObjectWrapper Structure") (Key :type String) (Value :type String) (FilePath :type "FilePath Structure"))
  (`|SetJsonField` JsonObject Key Value)
  (`JsonBlueprintFunctionLibrary.ToFile` JsonObject FilePath)
  (return))