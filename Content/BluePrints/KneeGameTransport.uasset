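; Transport actor for the knee game that receives webcam images and body joint angles from a TCP client.
; On client connection it caches the Webcam widget's image, if that widget exists, and sends the "knee_game" command.
; Received bytes are parsed as JSON to refresh the webcam display and set left vertical hip, vertical knee and lateral hip as main and sub angles.
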(event `self.ReceiveBeginPlay`
  (`parent.ReceiveBeginPlay`))

(event `self.TCPServer.OnClientConnected`
  (params (Client :type String))
  (bind _foundwidgets (`WidgetBlueprintLibrary.GetAllWidgetsOfClass` "/Game/MiniGame_KneeRehab/UI/Webcam.Webcam_C"))
  (if (`KismetArrayLibrary.Array_IsNotEmpty` _foundwidgets)
    (bind _image (`/Game/MiniGame_KneeRehab/UI/Webcam.GetImage` (`|GetArrayItem` _foundwidgets)))
    (set `self.Image` _image)
    (`self.SendCommand` "knee_game")))

(event `self.TCPServer.OnReceivedBytes`
  (params (Bytes :type "Array of Byte (by ref)"))
  (bind _returnvalue (`self.BytestreamToString` Bytes))
  (bind (_angle_l_vertical_hip _angle_l_lateral_hip _angle_l_vertical_knee _bodylength _incorrectjoint _image _error _success) (`self.ParseJson` _returnvalue))
  (if _success
    (`self.SetCurrentWebcamDisplay` _image)
    (`Image.SetBrushFromTexture` (`self.Image`) _image false)
    (`self.SetJointAngle` _angle_l_vertical_hip)
    (`self.SetSubAngle1` _angle_l_vertical_knee)
    (`self.SetSubAngle2` _angle_l_lateral_hip)))

(fn `UserConstructionScript`
  (`parent.UserConstructionScript`))