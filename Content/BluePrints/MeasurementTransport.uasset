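; Actor that runs body measurement over TCP, exchanging commands and results with a connected client.
; On connection it caches the GameUI widget's display image, and BeginMeasuring sends the "measuring_body" command.
; Received bytes are parsed as JSON, and successful parses push their image to that display.
; Once the body-length string is long enough, it stores the data, saves it through the UI and stops the thread.
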(event `self.ReceiveBeginPlay`
  (`parent.ReceiveBeginPlay`))

(event `self.TCPServer.OnClientConnected`
  (params (Client :type String))
  (bind _foundwidgets (`WidgetBlueprintLibrary.GetAllWidgetsOfClass` "/Game/MiniGame_KneeRehab/UI/GameUI.GameUI_C"))
  (if (not (`KismetArrayLibrary.Array_IsEmpty` _foundwidgets))
    (bind _output_get (set `self.MainUI` (`|GetArrayItem` _foundwidgets)))
    (bind _display (`/Game/MiniGame_KneeRehab/UI/GameUI.GetDisplay` _output_get))
    (set `self.Image` _display)))

(event `self.TCPServer.OnReceivedBytes`
  (params (Bytes :type "Array of Byte (by ref)"))
  (bind _returnvalue (`self.BytestreamToString` Bytes))
  (bind (_angle_l_vertical_hip _angle_l_lateral_hip _angle_l_vertical_knee _bodylength _incorrectjoint _image _error _success) (`self.ParseJson` _returnvalue true))
  (`KismetSystemLibrary.PrintString` (`KismetStringLibrary.Concat_StrStr` "Body Length : " _bodylength) false)
  (if _success
    (`Image.SetBrushFromTexture` (`self.Image`) _image false)
    (if (>= (`KismetStringLibrary.Len` _bodylength) 20)
      (`self.SetBodyData` _bodylength)
      (`/Game/MiniGame_KneeRehab/UI/GameUI.SaveUserData` (`self.MainUI`) _bodylength)
      (`self.StopThread`))))

(fn `BeginMeasuring`
  (`self.SendCommand` "measuring_body"))

(fn `UserConstructionScript`
  (`parent.UserConstructionScript`))